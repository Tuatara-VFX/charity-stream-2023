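; Collider actor that feeds its position, radius and velocity to a list of Niagara actors so their effects can react to it.
; Each Tick it derives velocity manually from the change in location, noted as a workaround for the editor, and draws a fixed-size debug sphere.
; It then writes the collider variables to each valid Niagara component, with radius scaled from the actor's largest scale axis.
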(event EventBeginPlay
  (Variables|Default|SetlastPosition (Transformation|GetActorLocation)))

(event Collision|EventActorBeginOverlap
  (params (OtherActor :type Actor%20Object%20Reference)))

(event EventTick
  (params (DeltaSeconds :type Float%20%28single-precision%29))
  (Rendering|Debug|DrawDebugSphere (Transformation|GetActorLocation) 5e+01 12 "(R=0.000000,G=1.000000,B=0.000000,A=0.500000)" 0.0)
  ;[1 1 1] Manual Velocity computation for Editor
  (if (Utilities|Operators|EqualEqual (Transformation|GetActorLocation) (Variables|Default|GetlastPosition) 0.0)
    (Variables|Default|Setvelocity "0, 0, 0")
    (else
      (Variables|Default|Setvelocity (/ (- (Transformation|GetActorLocation) (Variables|Default|GetlastPosition)) (Utilities|Time|GetWorldDeltaSeconds)))
      (Variables|Default|SetlastPosition (Transformation|GetActorLocation))))
  ;[1 1 1] Set Niagara Variables from Collider Actor
  (for _array_element (Variables|Default|GetNiagara%20Actors)
    (Utilities|IsValid _array_element
      (:Is%20Valid
        (Class|NiagaraComponent|SetVariablePosition (Variables|/Script/Niagara.NiagaraActor|GetNiagaraComponent _array_element) "Collider Position" (Transformation|GetActorLocation))
        (Niagara|SetNiagaraVariable(Float) (Variables|/Script/Niagara.NiagaraActor|GetNiagaraComponent _array_element) "Collider Radius" (* (Math|Vector|GetMaxElement (Transformation|GetActorScale3D)) 1e+02))
        (Niagara|SetNiagaraVariable(Vector3) (Variables|/Script/Niagara.NiagaraActor|GetNiagaraComponent _array_element) "Collider Velocity" (Variables|Default|Getvelocity))))))

(fn ConstructionScript)