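; Editor tool Blueprint that batch-generates randomized disk textures and saves them as static Texture2D assets.
; CreateTextures builds one render target and one transient dynamic material instance, then reuses both in a loop over the texture count.
; Each pass randomizes the background color, disk color and radius, draws the material to the target, and bakes it to an index-suffixed asset in the configured folder through an editor-only call.
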(fn ConstructionScript)

(fn CreateTextures
  ;[1 1 1] Preparation
  (bind _returnvalue (Rendering|CreateRenderTarget2D (Variables|Tool|GetWidth) (Variables|Tool|GetHeight) (Variables|Tool|GetRender%20Target%20Format) (Variables|Tool|GetClear%20Color)))
  (LocalVariables|SetRender%20Target _returnvalue)
  (bind _returnvalue_2 (Rendering|Material|CreateDynamicMaterialInstance (Variables|Tool|GetDraw%20Material) "None" "Transient" :!class /Script/Engine.KismetMaterialLibrary))
  (LocalVariables|SetDynamic%20Material _returnvalue_2)
  (for _index (range 1 (Variables|Tool|GetTexture%20Count))
    (Tool|ProcessandCreateStaticTexture (LocalVariables|GetRender%20Target) (Utilities|String|ToString(Integer) _index) (LocalVariables|GetDynamic%20Material))))

(fn ProcessandCreateStaticTexture
  (params (RenderTarget :type Texture%20Render%20Target%202D%20Object%20Reference) (Name%20Suffix :type String) (Material :type Material%20Instance%20Dynamic%20Object%20Reference))
  ;[1 1 1] Configure
  (Rendering|Material|SetVectorParameterValue Material "Background Color" (CallFunction|RandomColor) :!class /Script/Engine.MaterialInstanceDynamic)
  (Rendering|Material|SetVectorParameterValue Material "Disk Color" (CallFunction|RandomColor) :!class /Script/Engine.MaterialInstanceDynamic)
  (Rendering|Material|SetScalarParameterValue Material "Radius" (Math|Random|RandomFloatinRange 0.1 0.5) :!class /Script/Engine.MaterialInstanceDynamic)
  ;[1 1 1] Process
  (Rendering|DrawMaterialtoRenderTarget RenderTarget Material)
  ;[1 1 1] Output
  (Class|KismetRenderingLibrary|RenderTargetCreateStaticTexture2DEditorOnly RenderTarget (Utilities|String|Append (Variables|Tool|GetFolder) "/" (Variables|Tool|GetTexture%20Name) Name%20Suffix) (Variables|Tool|GetCompression%20Settings) "TMGS_FromTextureGroup"))

(fn RandomColor
  (return (Math|Color|MakeColor (Math|Random|RandomFloatinRange 0.0 1.0) (Math|Random|RandomFloatinRange 0.0 1.0) (Math|Random|RandomFloatinRange 0.0 1.0))))