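; BP_09_MakeGrid is an editor tool Blueprint that generates a grid texture asset.
; CreateTextures creates a render target from configurable size, format and clear color, then draws evenly spaced vertical and horizontal canvas lines based on cell counts.
; It then bakes the render target into a static Texture2D at the configured folder and name, using an editor-only function.
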(fn ConstructionScript)

(fn CreateTextures
  ;[1 1 1] Preparation
  (bind _returnvalue (Rendering|CreateRenderTarget2D (Variables|Tool|GetWidth) (Variables|Tool|GetHeight) (Variables|Tool|GetRender%20Target%20Format) (Variables|Tool|GetClear%20Color)))
  (bind _output_get (LocalVariables|SetRender%20Target _returnvalue))
  (bind _canvas (Rendering|BeginDrawCanvastoRenderTarget _output_get))
  (LocalVariables|SetDraw%20Canvas _canvas)
  (Utilities|FlowControl|Sequence
    (:then_0
      ;[1 1 1] Vertical lines
      (for _index (range 0 (Variables|Tool|GetX%20Cell%20Count))
        (Class|Canvas|DrawLine (LocalVariables|GetDraw%20Canvas) (Math|Vector2D|MakeVector2D (* (/ (Math|Conversions|ToFloat(Integer) (Variables|Tool|GetWidth)) (Math|Conversions|ToFloat(Integer) (Variables|Tool|GetX%20Cell%20Count))) _index) 0.0) (Math|Vector2D|MakeVector2D (* (/ (Math|Conversions|ToFloat(Integer) (Variables|Tool|GetWidth)) (Math|Conversions|ToFloat(Integer) (Variables|Tool|GetX%20Cell%20Count))) _index) (Math|Conversions|ToFloat(Integer) (Variables|Tool|GetHeight))) (Variables|Tool|GetLine%20Thickness) (Variables|Tool|GetLine%20Color))))
    (:then_1
      ;[1 1 1] Horizontal lines
      (for _index_2 (range 0 (Variables|Tool|GetY%20Cell%20Count))
        (Class|Canvas|DrawLine (LocalVariables|GetDraw%20Canvas) (Math|Vector2D|MakeVector2D 0.0 (* (/ (Math|Conversions|ToFloat(Integer) (Variables|Tool|GetHeight)) (Math|Conversions|ToFloat(Integer) (Variables|Tool|GetY%20Cell%20Count))) _index_2)) (Math|Vector2D|MakeVector2D (Math|Conversions|ToFloat(Integer) (Variables|Tool|GetWidth)) (* (/ (Math|Conversions|ToFloat(Integer) (Variables|Tool|GetHeight)) (Math|Conversions|ToFloat(Integer) (Variables|Tool|GetY%20Cell%20Count))) _index_2)) (Variables|Tool|GetLine%20Thickness) (Variables|Tool|GetLine%20Color))))
    (:then_2
      ;[1 1 1] Output
      (Class|KismetRenderingLibrary|RenderTargetCreateStaticTexture2DEditorOnly (LocalVariables|GetRender%20Target) (Utilities|String|Append (Variables|Tool|GetFolder) "/" (Variables|Tool|GetTexture%20Name)) (Variables|Tool|GetCompression%20Settings) "TMGS_FromTextureGroup"))))