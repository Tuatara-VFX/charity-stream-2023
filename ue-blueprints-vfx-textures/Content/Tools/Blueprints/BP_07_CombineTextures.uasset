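; BP_07_CombineTextures is an editor tool that combines Red, Green and Blue input textures into a single saved texture asset.
; CreateTextures makes a render target and a transient dynamic instance of DrawMaterial, then feeds the three textures in as parameters.
; It draws that material to the render target and bakes the result into a static Texture2D with configurable folder, name and compression, using an editor-only call.
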(fn ConstructionScript)

(fn CreateTextures
  ;[1 1 1] Preparation
  (bind _returnvalue (Rendering|CreateRenderTarget2D (Variables|Tool|GetWidth) (Variables|Tool|GetHeight) (Variables|Tool|GetRender%20Target%20Format) (Variables|Tool|GetClear%20Color)))
  (LocalVariables|SetRender%20Target _returnvalue)
  (bind _returnvalue_2 (Rendering|Material|CreateDynamicMaterialInstance (Variables|Tool|GetDraw%20Material) "None" "Transient" :!class /Script/Engine.KismetMaterialLibrary))
  (LocalVariables|SetDynamic%20Material _returnvalue_2)
  ;[1 1 1] Configure
  (Rendering|Material|SetTextureParameterValue (LocalVariables|GetDynamic%20Material) "Red" (Variables|Tool|GetRed))
  (Rendering|Material|SetTextureParameterValue (LocalVariables|GetDynamic%20Material) "Green" (Variables|Tool|GetGreen))
  (Rendering|Material|SetTextureParameterValue (LocalVariables|GetDynamic%20Material) "Blue" (Variables|Tool|GetBlue))
  ;[1 1 1] Process
  (Rendering|DrawMaterialtoRenderTarget (LocalVariables|GetRender%20Target) (LocalVariables|GetDynamic%20Material))
  ;[1 1 1] Output
  (Class|KismetRenderingLibrary|RenderTargetCreateStaticTexture2DEditorOnly (LocalVariables|GetRender%20Target) (Utilities|String|Append (Variables|Tool|GetFolder) "/" (Variables|Tool|GetTexture%20Name)) (Variables|Tool|GetCompression%20Settings) "TMGS_FromTextureGroup"))