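; Editor tool Blueprint that splits a source texture's R, G, B and A channels into four separate static texture assets.
; CreateTextures builds one render target and a transient dynamic material from DrawMaterial, then runs ProcessOneChannel once per channel.
; Each pass sets the texture and channel mask, draws to the shared target and bakes it via editor-only static texture creation, named from folder, base name and channel suffix.
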(fn ConstructionScript)

(fn CreateTextures
  ;[1 1 1] Preparation
  (bind _returnvalue (Rendering|CreateRenderTarget2D (Variables|Tool|GetWidth) (Variables|Tool|GetHeight) (Variables|Tool|GetRender%20Target%20Format) (Variables|Tool|GetClear%20Color)))
  (LocalVariables|SetRender%20Target _returnvalue)
  (bind _returnvalue_2 (Rendering|Material|CreateDynamicMaterialInstance (Variables|Tool|GetDraw%20Material) "None" "Transient" :!class /Script/Engine.KismetMaterialLibrary))
  (LocalVariables|SetDynamic%20Material _returnvalue_2)
  (Utilities|FlowControl|Sequence
    (:then_0
      (CallFunction|ProcessOneChannel (LocalVariables|GetRender%20Target) (LocalVariables|GetDynamic%20Material) "_R" (Math|Vector4|MakeVector4 1.0 0.0 0.0 0.0)))
    (:then_1
      (CallFunction|ProcessOneChannel (LocalVariables|GetRender%20Target) (LocalVariables|GetDynamic%20Material) "_G" (Math|Vector4|MakeVector4 0.0 1.0 0.0 0.0)))
    (:then_2
      (CallFunction|ProcessOneChannel (LocalVariables|GetRender%20Target) (LocalVariables|GetDynamic%20Material) "_B" (Math|Vector4|MakeVector4 0.0 0.0 1.0 0.0)))
    (:then_3
      (CallFunction|ProcessOneChannel (LocalVariables|GetRender%20Target) (LocalVariables|GetDynamic%20Material) "_A" (Math|Vector4|MakeVector4 0.0 0.0 0.0 1.0)))))

(fn ProcessOneChannel
  (params (Render%20Target :type Texture%20Render%20Target%202D%20Object%20Reference) (Dynamic%20Material :type Material%20Instance%20Dynamic%20Object%20Reference) (Texture%20Name%20Suffix :type String) (Mask :type Vector%204%20Structure))
  ;[1 1 1] Configure
  (Rendering|Material|SetTextureParameterValue Dynamic%20Material "MainTex" (Variables|Tool|GetTexture))
  (Rendering|Material|SetVectorParameterValue Dynamic%20Material "Mask" (Utilities|Struct|MakeLinearColor (.x Mask) (.y Mask) (.z Mask) (.w Mask)) :!class /Script/Engine.MaterialInstanceDynamic)
  ;[1 1 1] Process
  (Rendering|DrawMaterialtoRenderTarget Render%20Target Dynamic%20Material)
  ;[1 1 1] Output
  (Class|KismetRenderingLibrary|RenderTargetCreateStaticTexture2DEditorOnly Render%20Target (Utilities|String|Append (Variables|Tool|GetFolder) "/" (Variables|Tool|GetTexture%20Name) Texture%20Name%20Suffix) (Variables|Tool|GetCompression%20Settings) "TMGS_FromTextureGroup"))