(fn ConstructionScript)

(fn CreateTexture
  ;[1 1 1] Preparation
  (bind _returnvalue (Rendering|CreateRenderTarget2D (Variables|Tool|GetWidth) (Variables|Tool|GetHeight) (Variables|Tool|GetRender%20Target%20Format) (Variables|Tool|GetClear%20Color)))
  (LocalVariables|SetRender%20Target _returnvalue)
  ;[0.5453 1 0.4133] Process
  (Rendering|DrawMaterialtoRenderTarget (LocalVariables|GetRender%20Target) (Variables|Tool|GetDraw%20Material))
  ;[1 1 1] Output
  (Class|KismetRenderingLibrary|RenderTargetCreateStaticTexture2DEditorOnly (LocalVariables|GetRender%20Target) (Utilities|String|Append (Variables|Tool|GetFolder) "/" (Variables|Tool|GetTexture%20Name)) (Variables|Tool|GetCompression%20Settings) "TMGS_FromTextureGroup"))